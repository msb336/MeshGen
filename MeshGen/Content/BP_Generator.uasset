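; BP_Generator is an actor that displays procedurally generated geometry through its GeneratedMesh procedural mesh.
; The construction script builds the mesh section from the Vertices and Index arrays.
; Each Tick calls Update, whose logic is not in these graphs, and recreates the section from those arrays when it returns true.
; The overlap event is empty, and a disconnected Count increment never runs.
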(event Collision|EventActorBeginOverlap
  (params (OtherActor :type Actor%20Object%20Reference)))

(event EventTick
  (params (DeltaSeconds :type Float%20%28single-precision%29))
  (bind _returnvalue (Class|Generator|Update))
  (if _returnvalue
    (Class|ProceduralMeshComponent|CreateMeshSectionLinearColor (Variables|Default|GetGeneratedMesh) 0 (Variables|Default|Getvertices_) (Variables|Default|Getindex_) 0 0 0 0 false)))

(fn ConstructionScript
  (Class|ProceduralMeshComponent|CreateMeshSectionLinearColor (Variables|Default|GetGeneratedMesh) 0 (Variables|Default|Getvertices_) (Variables|Default|Getindex_) 0 0 0 0 false))