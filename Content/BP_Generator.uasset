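; BP_Generator is an actor that builds a procedural mesh from its vertex, triangle and UV arrays.
; On BeginPlay it applies the generated material, calls Update, then, guarded by GenCalled, prints the result and creates the mesh section with UVs and collision.
; The construction script also creates a section from the vertices and triangles alone, without UVs or explicitly enabled collision.
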(event EventBeginPlay
  (Rendering|Material|SetMaterial (Variables|Default|GetGeneratedMesh) 0 "/MeshGen/generated_material.generated_material")
  (bind _returnvalue (Class|Generator|Update))
  (if (not (Variables|Default|Getgen_called_))
    (Development|PrintString _returnvalue)
    (Variables|Default|Setgen_called_ true)
    (Class|ProceduralMeshComponent|CreateMeshSectionLinearColor (Variables|Default|GetGeneratedMesh) 0 (Variables|Default|Getvertices_) (Variables|Default|Getindex_) 0 (Variables|Default|Getuvs_) 0 0 0 0 0 true)))

(event Collision|EventActorBeginOverlap
  (params (OtherActor :type Actor%20Object%20Reference)))

(event EventTick
  (params (DeltaSeconds :type Float%20%28single-precision%29)))

(fn ConstructionScript
  (Class|ProceduralMeshComponent|CreateMeshSectionLinearColor (Variables|Default|GetGeneratedMesh) 0 (Variables|Default|Getvertices_) (Variables|Default|Getindex_) 0 0 0 0 0 0 0 false))